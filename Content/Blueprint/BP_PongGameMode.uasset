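; Game mode for a Pong game that creates the score HUD, tracks both players' scores and spawns the ball.
; On BeginPlay it picks a random horizontal serve direction, then spawns a ball and launches it along X with physics velocity after short delays.
; Each scoring event increments that player's score, updates the HUD, sets the next serve direction by scorer and spawns another ball.
; The two UpdatePlayerScoreServer events are empty stubs.
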(event Custom|IncreasePlayerTwoScoreServer
  ;[1 1 1] Add score functions
  (bind _result (Math|Integer|IncrementInt (Variables|Default|Getm_playerTwoScore))
    (:%20%20
      (Class|GameHud|UpdatePlayerTwoScore (Variables|Default|Getm_gameHudRef) _result)
      (Development|PrintString (Utilities|String|ToString(Integer) _result))
      (Variables|Default|Setm_direction -1.0)
      (Class|PongGameMode|SpawnNewBall))))

(event Custom|IncreasePlayerOneScoreServer
  ;[1 1 1] Add score functions
  (bind _result (Math|Integer|IncrementInt (Variables|Default|Getm_playerOneScore))
    (:%20%20
      (Class|GameHud|UpdatePlayerOneScore (Variables|Default|Getm_gameHudRef) _result)
      (Development|PrintString (Utilities|String|ToString(Integer) _result) true true "(R=1.000000,G=0.000000,B=0.026767,A=1.000000)")
      (Variables|Default|Setm_direction 1.0)
      (Class|PongGameMode|SpawnNewBall))))

(event Custom|UpdatePlayerOneScoreServer
  ;[1 1 1] Update the score
)

(event Custom|UpdatePlayerTwoScoreServer
  ;[1 1 1] Update the score
)

(event EventBeginPlay
  ;[1 1 1] Set references, create widget and set ball speed
  (bind _returnvalue (UserInterface|CreateWidget "/Game/Blueprint/WBP_GameHud.WBP_GameHud_C"))
  (bind _output_get (Variables|Default|Setm_gameHudRef _returnvalue))
  (UserInterface|Viewport|AddtoViewport _output_get 0)
  (Variables|Default|Setm_direction (Math|Float|Sign(Float) (Math|Random|RandomFloatinRange -1.0 1.0)))
  (Class|PongGameMode|SpawnNewBall))

(event EventSpawnNewBall
  ;[1 1 1] Spawn Ball
  (Utilities|FlowControl|Delay 1.0)
  (bind _returnvalue (Game|SpawnActorfromClass "/Game/Blueprint/BP_Ball.BP_Ball_C" (Math|Transform|MakeTransform "0,10.000000, 0" "0, 0, 0" "1,1,1") "AlwaysSpawn" 0 0))
  (bind _output_get (Variables|Default|Setm_ballRef _returnvalue))
  (Utilities|FlowControl|Delay 0.5)
  (Physics|SetPhysicsLinearVelocity (Variables|/Script/Pong.Ball|Getsphere _output_get) (Math|Vector|MakeVector (* (Variables|Default|Getm_direction) (Variables|Default|Getm_ballSpeed)) 0.0 0.0) false "None"))

(event EventIncreasePlayerOneScore
  ;[1 1 1] Add score functions
  (CallFunction|IncreasePlayerOneScoreServer))

(event EventIncreasePlayerTwoScore
  ;[1 1 1] Add score functions
  (CallFunction|IncreasePlayerTwoScoreServer))

(fn ConstructionScript)