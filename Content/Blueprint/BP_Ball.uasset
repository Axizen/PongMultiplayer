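; BP_Ball is a physics-driven ball that bounces off paddles and boundaries, in the style of Pong.
; Overlaps are handled only on authority, with casts to Paddle or Boundary choosing the response.
; A paddle hit reverses X and derives Z from the paddle collider's scaled velocity plus random variation.
; A boundary hit reverses Z with random variation, setting the Sphere's velocity directly in both cases.
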(event EventHitPaddle
  (params (paddle :type Paddle%20Object%20Reference))
  ;[1 1 1] Hit Paddle Functionality
  (bind _returnvalue (Physics|GetPhysicsLinearVelocity (Variables|/Script/Pong.Paddle|Getcollider paddle) "None"))
  (bind _returnvalue_2 (Physics|GetPhysicsLinearVelocity (Variables|Default|Getsphere) "None"))
  (Physics|SetPhysicsLinearVelocity (Variables|Default|Getsphere) (Math|Vector|MakeVector (* (.x _returnvalue_2) -1.0) (.y _returnvalue_2) (+ (/ (.z _returnvalue) (Math|Random|RandomFloatinRange 2.0 3.0)) (Math|Random|RandomFloatinRange -2e+02 2e+02))) false "None"))

(event Collision|EventActorBeginOverlap
  (params (OtherActor :type Actor%20Object%20Reference))
  ;[1 1 1] Collision Check
  (Networking|SwitchHasAuthority
    (:Authority
      (bind _aspaddle (Utilities|Casting|CastToPaddle OtherActor)
        (:then
          (Class|Ball|HitPaddle _aspaddle))
        (:CastFailed
          (Utilities|Casting|CastToBoundary OtherActor)
          (Class|Ball|HitBoundary))))))

(event EventHitBoundary
  ;[1 1 1] Hit Boundary Functionality
  (bind _returnvalue (Physics|GetPhysicsLinearVelocity (Variables|Default|Getsphere) "None"))
  (Physics|SetPhysicsLinearVelocity (Variables|Default|Getsphere) (Math|Vector|MakeVector (.x _returnvalue) (.y _returnvalue) (+ (* (.z _returnvalue) -1.0) (Math|Random|RandomFloatinRange -2e+02 2e+02))) false "None"))

(fn ConstructionScript)